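; Rabbit character pawn that walks or sprints and deals heavy damage to actors it runs into.
; BeginSprint and EndSprint switch walk speed and the sprint flag, which enables a short per-tick forward trace from the spine socket to damage blockers.
; Capsule hits apply the same damage regardless of sprinting.
; CanSeePlayerPawn line-traces forward over SightLength, reporting whether the hit actor is tagged Player; both traces draw debug lines.
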(event OnComponentHit(CapsuleComponent)
  (params (HitComponent :type Primitive%20Component%20Object%20Reference) (OtherActor :type Actor%20Object%20Reference) (OtherComp :type Primitive%20Component%20Object%20Reference) (NormalImpulse :type Vector :default "0, 0, 0") (Hit :type Hit%20Result%20Structure%20%28by%20ref%29))
  (Game|Damage|ApplyDamage OtherActor 1e+02 0 0))

(event EventBeginPlay
  (Variables|/Script/Engine.CharacterMovementComponent|SetMaxWalkSpeed (Variables|Character|GetCharacterMovement) (Variables|Pawn|Character|GetWalkGroundSpeed)))

(event Collision|EventActorBeginOverlap
  (params (OtherActor :type Actor%20Object%20Reference)))

(event EventTick
  (params (DeltaSeconds :type Float%20%28single-precision%29))
  (bind _mesh (Variables|Character|GetMesh))
  (bind _returnvalue (Transformation|GetSocketLocation _mesh "spine"))
  (if (Variables|Default|GetIsSprinting)
    (bind _outhit (Collision|LineTraceByChannel _returnvalue (+ _returnvalue (* (Transformation|GetActorForwardVector) 5e+01)) "TraceTypeQuery3" false 0 "ForOneFrame"))
    (if (.bBlockingHit (Collision|BreakHitResult _outhit))
      (Game|Damage|ApplyDamage (.HitActor (Collision|BreakHitResult _outhit)) 1e+02 0 0))))

(fn ConstructionScript)

(fn CanSeePlayerPawn
  (bind _returnvalue (Transformation|GetActorLocation))
  (bind (_outhit _returnvalue_2) (Collision|LineTraceByChannel _returnvalue (+ _returnvalue (* (Transformation|GetActorForwardVector) (Variables|Pawn|Character|GetSightLength))) "TraceTypeQuery3" false 0 "ForOneFrame"))
  (if _returnvalue_2
    (LocalVariables|SetIsPlayer (Actor|ActorHasTag (.HitActor (Collision|BreakHitResult _outhit)) "Player"))
    (LocalVariables|SetTargetActor (.HitActor (Collision|BreakHitResult _outhit)))
    (else
      (LocalVariables|SetIsPlayer false)))
  (return (LocalVariables|GetIsPlayer) (LocalVariables|GetTargetActor)))

(fn BeginSprint
  (Variables|Default|SetIsSprinting true)
  (Variables|/Script/Engine.CharacterMovementComponent|SetMaxWalkSpeed (Variables|Character|GetCharacterMovement) (Variables|Pawn|Character|GetSprintGroundSpeed)))

(fn EndSprint
  (Variables|/Script/Engine.CharacterMovementComponent|SetMaxWalkSpeed (Variables|Character|GetCharacterMovement) (Variables|Pawn|Character|GetWalkGroundSpeed))
  (Variables|Default|SetIsSprinting false))